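; Base interactable weapon that sends an equip message to whoever interacts with it and handles firing and reloading.
; Fire spawns a BP_BaseProjectile at the muzzle socket, decrements ammo and plays WeaponInfo effects, relying on player 0's character having an equipped item.
; Reload refills from reserve ammo, discarding rounds left in the magazine.
; An unconnected line-trace radial-damage path never runs.
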(event `/Game/Interactables/BPI_Interact.Interaction`
  (params (Instigator :type "Object Object Reference"))
  (message `/Game/Interactables/BPI_Interact.Equip` Instigator self (`self.ItemInfo`)))

(event `Fire`
  (bind (_weaponinfo_attacktype _weaponinfo_damage _weaponinfo_range _weaponinfo_attackspeed _weaponinfo_attachsocket _weaponinfo_attackvisualeffects _weaponinfo_attacksoundeffects) (break `/Game/Interactables/Weapons/F_WeaponInfo` (`self.WeaponInfo`)))
  ;[1 1 1] Fire's weapon projectile from socket
  (if (== (`self.Ammo`) 0)
    (`KismetSystemLibrary.PrintString` "Out Of Ammo!")
    (else
      (bind _asthird_person_character (cast `/Game/ThirdPersonBP/Blueprints/ThirdPersonCharacter` (`GameplayStatics.GetPlayerCharacter` 0)))
      (if (`KismetSystemLibrary.IsValid` (`/Game/ThirdPersonBP/Blueprints/ThirdPersonCharacter.EquippedItem` _asthird_person_character))
        (`|SpawnActorFromClass` "/Game/Interactables/Weapons/BP_BaseProjectile.BP_BaseProjectile_C" (`SceneComponent.GetSocketTransform` (`self.InteractableMesh`) "Gun Exit Socket" "RTS_World") "Undefined" "OverrideRootScale" null null)
        (set `self.Ammo` (- (`self.Ammo`) 1))
        (bind _asthird_person_character_2 (cast `/Game/ThirdPersonBP/Blueprints/ThirdPersonCharacter` (`GameplayStatics.GetPlayerCharacter` 0)))
        (bind _interactablemesh (`/Game/Interactables/BP_BaseInteractable.InteractableMesh` (`/Game/ThirdPersonBP/Blueprints/ThirdPersonCharacter.EquippedItem` _asthird_person_character_2)))
        (bind _returnvalue (`GameplayStatics.SpawnEmitterAtLocation` _weaponinfo_attackvisualeffects (`SceneComponent.GetSocketLocation` _interactablemesh "Gun Exit Socket") (`SceneComponent.GetSocketRotation` _interactablemesh "Gun Exit Socket")))
        (`SceneComponent.SetWorldScale3D` _returnvalue (0.5 0.5 0.5))
        (`GameplayStatics.PlaySound2D` _weaponinfo_attacksoundeffects)))))

(fn `GetWeaponInfo`
  (returns (WeaponInfo :type "/Game/Interactables/Weapons/F_WeaponInfo Structure"))
  (return (`self.WeaponInfo`)))

(fn `Reload`
  (bind (_weaponinfo_attacktype _weaponinfo_damage _weaponinfo_range _weaponinfo_attackspeed _weaponinfo_attachsocket _weaponinfo_attackvisualeffects _weaponinfo_attacksoundeffects _weaponinfo_hitvisualeffects _weaponinfo_hitsoundeffects _weaponinfo_attackmonatage _weaponinfo_weaponclasstype _weaponinfo_weaponkind _weaponinfo_durability _weaponinfo_magsize) (break `/Game/Interactables/Weapons/F_WeaponInfo` (`self.WeaponInfo`)))
  (bind (_weaponinfo_attacktype_2 _weaponinfo_damage_2 _weaponinfo_range_2 _weaponinfo_attackspeed_2 _weaponinfo_attachsocket_2 _weaponinfo_attackvisualeffects_2 _weaponinfo_attacksoundeffects_2 _weaponinfo_hitvisualeffects_2 _weaponinfo_hitsoundeffects_2 _weaponinfo_attackmonatage_2 _weaponinfo_weaponclasstype_2 _weaponinfo_weaponkind_2 _weaponinfo_durability_2 _weaponinfo_magsize_2) (break `/Game/Interactables/Weapons/F_WeaponInfo` (`self.WeaponInfo`)))
  (bind (_weaponinfo_attacktype_3 _weaponinfo_damage_3 _weaponinfo_range_3 _weaponinfo_attackspeed_3 _weaponinfo_attachsocket_3 _weaponinfo_attackvisualeffects_3 _weaponinfo_attacksoundeffects_3 _weaponinfo_hitvisualeffects_3 _weaponinfo_hitsoundeffects_3 _weaponinfo_attackmonatage_3 _weaponinfo_weaponclasstype_3 _weaponinfo_weaponkind_3 _weaponinfo_durability_3 _weaponinfo_magsize_3) (break `/Game/Interactables/Weapons/F_WeaponInfo` (`self.WeaponInfo`)))
  (bind (_weaponinfo_attacktype_4 _weaponinfo_damage_4 _weaponinfo_range_4 _weaponinfo_attackspeed_4 _weaponinfo_attachsocket_4 _weaponinfo_attackvisualeffects_4 _weaponinfo_attacksoundeffects_4 _weaponinfo_hitvisualeffects_4 _weaponinfo_hitsoundeffects_4 _weaponinfo_attackmonatage_4 _weaponinfo_weaponclasstype_4 _weaponinfo_weaponkind_4 _weaponinfo_durability_4 _weaponinfo_magsize_4) (break `/Game/Interactables/Weapons/F_WeaponInfo` (`self.WeaponInfo`)))
  (if (== _weaponinfo_magsize (`self.Ammo`))
    _
    (elif (>= (`self.MaxAmmo`) _weaponinfo_magsize_4)
      (set `self.Ammo` _weaponinfo_magsize_2)
      (set `self.MaxAmmo` (- (`self.MaxAmmo`) _weaponinfo_magsize_3))
      (else
        (set `self.Ammo` (`self.MaxAmmo`))
        (set `self.MaxAmmo` 0)))))

(fn `UserConstructionScript`
  (`parent.UserConstructionScript`))