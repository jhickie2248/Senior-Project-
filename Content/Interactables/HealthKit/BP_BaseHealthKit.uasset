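; Base health kit interactable that restores health to the player character.
; HealPlayer casts player 0 to ThirdPersonCharacter and, if below max health, adds HealthInfo's heal amount without clamping, then calls CallUpdateHealth with the new value.
; The event graph holds only disabled stub events, so nothing here triggers the heal, and GetHealthKitInfo has an empty body.
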(fn `Get Health Kit Info`
  (returns (`Health Kit Info` :type "/Game/Interactables/HealthKit/F_HealthKitInfo Structure"))
  (return))

(fn `Heal Player`
  (bind _health_info_healthtoheal (break `/Game/Interactables/HealthKit/F_HealthKitInfo` (`self.Health Info`)))
  (bind _asthird_person_character (cast `/Game/ThirdPersonBP/Blueprints/ThirdPersonCharacter` (`GameplayStatics.GetPlayerCharacter` 0)))
  (bind _playercurrenthealth (`/Game/ThirdPersonBP/Blueprints/ThirdPersonCharacter.PlayerCurrentHealth` _asthird_person_character))
  (if (< _playercurrenthealth (`/Game/ThirdPersonBP/Blueprints/ThirdPersonCharacter.PlayerMaxHealth` _asthird_person_character))
    (bind _output_get (set `/Game/ThirdPersonBP/Blueprints/ThirdPersonCharacter.PlayerCurrentHealth` (+ _playercurrenthealth _health_info_healthtoheal) _asthird_person_character))
    (`/Game/ThirdPersonBP/Blueprints/ThirdPersonCharacter.UpdateHealth` _asthird_person_character _output_get)))

(fn `UserConstructionScript`
  (`parent.UserConstructionScript`))