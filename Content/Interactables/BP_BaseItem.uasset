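; BP_BaseItem is a base pickup item that a ThirdPersonCharacter collects by interacting with it.
; On interaction it passes its ItemInfo struct to the character through PickupMessage, then destroys itself.
; The construction script rebuilds ItemInfo with the actor's own class, so each item identifies its class automatically while keeping its type, name, image, index and socket.
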(event `/Game/Interactables/BPI_Interact.Interaction`
  (params (Instigator :type "Object Object Reference"))
  (cast `/Game/ThirdPersonBP/Blueprints/ThirdPersonCharacter` Instigator)
  (if true
    (message `/Game/Interactables/BPI_Interact.Pickup` Instigator (`self.ItemInfo`))
    (`self.K2_DestroyActor`)))

(fn `UserConstructionScript`
  (bind (_iteminfo_itemtype _iteminfo_itemname _iteminfo_itemimage _iteminfo_itemclass _iteminfo_itemindex _iteminfo_itemsocket) (break `/Game/Interactables/F_ItemInfo` (`self.ItemInfo`)))
  ;[1 1 1] Makes it automatically Identify Object Class
  (`parent.UserConstructionScript`)
  (set `self.ItemInfo` (make `/Game/Interactables/F_ItemInfo` _iteminfo_itemtype _iteminfo_itemname _iteminfo_itemimage (`GameplayStatics.GetObjectClass` self) _iteminfo_itemindex _iteminfo_itemsocket)))