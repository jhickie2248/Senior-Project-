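; Base AI enemy character that roams, patrols or chases the player and is destroyed when its health runs out.
; AIState picks a looping AIMoveTo behavior at BeginPlay, while PawnSensing triggers a chase that damages the player on arrival and repeats.
; Player death disables sensing updates and reruns the state behavior.
; Projectile overlaps deal equipped-weapon damage only if its class matches EnemyDamagedBy, whereas AnyDamage subtracts unconditionally and updates health.
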(event `self.CapsuleComponent.OnComponentBeginOverlap`
  (params (OverlappedComponent :type "PrimitiveComponent Object Reference") (OtherActor :type "Actor Object Reference") (OtherComp :type "PrimitiveComponent Object Reference") (OtherBodyIndex :type Integer) (bFromSweep :type Boolean) (SweepResult :type "HitResult Structure (by ref)"))
  (bind (_enemyinfo_enemystate _enemyinfo_enemytype _enemyinfo_attackvisualeffects _enemyinfo_enemydamagedby) (break `/Game/AI/F_EnemyInfo` (`self.EnemyInfo`)))
  (bind _asthird_person_character (cast `/Game/ThirdPersonBP/Blueprints/ThirdPersonCharacter` (`GameplayStatics.GetPlayerCharacter` 0)))
  (bind _equippeditem (`/Game/ThirdPersonBP/Blueprints/ThirdPersonCharacter.EquippedItem` _asthird_person_character))
  (bind _iteminfo_itemtype (break `/Game/Interactables/F_ItemInfo` (`/Game/Interactables/BP_BaseItem.ItemInfo` _equippeditem)))
  (if (and (`KismetSystemLibrary.IsValid` _equippeditem) (`|EnumEquality` _iteminfo_itemtype "NewEnumerator2"))
    (bind _weaponinfo (message `/Game/Interactables/Weapons/I_Weapon.GetWeaponInfo` _equippeditem))
    (cast `/Game/Interactables/Weapons/BP_BaseProjectile` OtherActor)
    ;[1 1 1] Test String
    (`KismetSystemLibrary.PrintString` "Hit")
    (if (`|EnumEquality` _enemyinfo_enemydamagedby (`.WeaponClassType_58_5D169C5B40870F073F1BFCA7BDDE7F71` (break `/Game/Interactables/Weapons/F_WeaponInfo` _weaponinfo)))
      (set `self.EnemyCurrentHealth` (- (`self.EnemyCurrentHealth`) (`.Damage_5_4BBAAB1B4C66716D9AB3E49C17A40B1A` (break `/Game/Interactables/Weapons/F_WeaponInfo` _weaponinfo))))
      (if (<= (`self.EnemyCurrentHealth`) 0.0)
        (`self.K2_DestroyActor`)))))

(event `self.ReceiveBeginPlay`
  ;[1 1 1] Contrls for which action
  (bind _asthird_person_character (cast `/Game/ThirdPersonBP/Blueprints/ThirdPersonCharacter` (`GameplayStatics.GetPlayerCharacter` 0)))
  (add `/Game/ThirdPersonBP/Blueprints/ThirdPersonCharacter.PlayerDead` _asthird_person_character (delegate `ResetAI`))
  (switch `/Game/AI/E_AIState` (`self.AIState`)
    (:`NewEnumerator1`
      (`self.Move to Random Location`))
    (:`NewEnumerator2`
      (`self.CHase Player` null))
    (:`NewEnumerator3`
      (`self.Patrol`))))

(event `ResetAI`
  ;[1 1 1] Contrls for which action
  (`PawnSensingComponent.SetSensingUpdatesEnabled` (`self.PawnSensing`) false)
  (switch `/Game/AI/E_AIState` (`self.AIState`)
    (:`NewEnumerator1`
      (`self.Move to Random Location`))
    (:`NewEnumerator2`
      (`self.CHase Player` null))
    (:`NewEnumerator3`
      (`self.Patrol`))))

(event `self.ReceiveAnyDamage`
  (params (Damage :type "Float (single-precision)") (DamageType :type "DamageType Object Reference") (InstigatedBy :type "Controller Object Reference") (DamageCauser :type "Actor Object Reference"))
  ;[1 1 1] Failed damae by line trace
  (if true
    (bind _output_get (set `self.EnemyCurrentHealth` (- (`self.EnemyCurrentHealth`) Damage)))
    (`self.Update Enemy Health`)
    (if (<= _output_get 0.0)
      (`self.K2_DestroyActor`))))

(event `Move to Random Location`
  ;[1 1 1] Makes Acter move to random location (Roam)
  (`|AIMoveTo` self (`NavigationSystem.K2_GetRandomLocationInNavigableRadius` (`self.K2_GetActorLocation`) 500.0)
    (:`OnSuccess`
      (`KismetSystemLibrary.Delay` 1.0)
      (`self.Move to Random Location`))))

(event `CHase Player`
  (params (PlayerToChase :type "Pawn Object Reference"))
  ;[1 1 1] Chases after player and "self destruct" when in reach
  (if (`PawnSensingComponent.bEnableSensingUpdates` (`self.PawnSensing`))
    (`|AIMoveTo` self (0.0 0.0 0.0) PlayerToChase
      (:`OnSuccess`
        (`GameplayStatics.ApplyDamage` PlayerToChase (`self.Damage`))
        (`KismetSystemLibrary.Delay` 1.0)
        (`self.CHase Player` PlayerToChase)))))

(event `Patrol`
  ;[1 1 1] Patrol between target points
  (`|AIMoveTo` self (0.0 0.0 0.0) (`self.TargetPoint1`)
    (:`OnSuccess`
      (`KismetSystemLibrary.Delay` 3.0)
      (`|AIMoveTo` self (0.0 0.0 0.0) (`self.TargetPoint2`)
        (:`OnSuccess`
          (`KismetSystemLibrary.Delay` 3.0)
          (`self.Patrol`))))))

(event `self.PawnSensing.OnSeePawn`
  (params (Pawn :type "Pawn Object Reference"))
  ;[1 1 1] Chase Player When in sight
  (bind _asthird_person_character (cast `/Game/ThirdPersonBP/Blueprints/ThirdPersonCharacter` Pawn))
  (`self.CHase Player` _asthird_person_character))

(fn `UserConstructionScript`)